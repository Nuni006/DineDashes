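; Player car Blueprint for driving with delivery missions, handling vehicle input, camera, music toggle and pause menu.
; Input feeds throttle, brake, steering and handbrake to the movement component, while the mouse rotates the spring arm.
; BeginPlay creates the delivery text widget, updated by NovaMisija, and an M-toggled map.
; Tick, throttled by a Delay, converts world location into a clamped map position.
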(event Custom|ToggleMusic
  (bind _music (Variables|Default|GetMusic))
  (bind _output_get (Variables|Default|SetMuskaJe (not (Variables|Default|GetMuskaJe))))
  (if _output_get
    (Audio|Components|Audio|SetVolumeMultiplier _music 0.0 :!class /Script/Engine.AudioComponent)
    (else
      (Audio|Components|Audio|SetVolumeMultiplier _music 1.0 :!class /Script/Engine.AudioComponent)
      (Audio|Components|Audio|Play _music 0.0))))

(event Collision|EventActorBeginOverlap
  (params (OtherActor :type Actor%20Object%20Reference)))

(event EventBeginPlay
  (bind _returnvalue (UserInterface|CreateWidget "/Game/dostave/DostaveTXTWidget.DostaveTXTWidget_C" (Game|GetPlayerController 0)))
  (bind _output_get (Variables|Default|SetDostavaWidget _returnvalue))
  (UserInterface|Viewport|AddtoViewport _output_get 0)
  (bind _returnvalue_2 (UserInterface|CreateWidget "/Game/mapca/Mapa.Mapa_C" (Game|GetPlayerController 0)))
  (bind _output_get_2 (Variables|Default|SetMapcaUI _returnvalue_2))
  (UserInterface|Viewport|AddtoViewport _output_get_2 0)
  (Widget|SetVisibility (Variables|Default|GetMapcaUI) "Collapsed"))

(event EventTick
  (params (DeltaSeconds :type Float%20%28single-precision%29))
  (bind _returnvalue (Transformation|GetActorLocation))
  (Utilities|FlowControl|Delay 0.1)
  (Default|NastaviPozicijo (Variables|Default|GetMapcaUI) (Math|Vector2D|MakeVector2D (Math|Float|Clamp(Float) (* (/ (.x _returnvalue) 2e+05) -1e+03) -5e+02 5e+02) (Math|Float|Clamp(Float) (* (/ (.y _returnvalue) 2e+05) -1e+03) -5e+02 5e+02))))

(event Input|ActionEvents|InputActionRocna
  (params (Key :type Key%20Structure :default "None"))
  (bind _vehiclemovementcomponent (Variables|Default|GetVehicleMovementComponent))
  (:Pressed
    (Class|ChaosVehicleMovementComponent|SetHandbrakeInput _vehiclemovementcomponent true))
  (:Released
    (Class|ChaosVehicleMovementComponent|SetHandbrakeInput _vehiclemovementcomponent false)))

(event Input|ActionEvents|InputActionPause
  (params (Key :type Key%20Structure :default "None"))
  (:Pressed
    (bind _returnvalue (UserInterface|CreateWidget "/Game/UI/PauseMenu.PauseMenu_C"))
    (UserInterface|Viewport|AddtoViewport _returnvalue 0)
    (Game|SetGamePaused true)
    (Input|SetInputModeUIOnly (Game|GetPlayerController 0) _returnvalue "DoNotLock" false)))

(event Input|AxisEvents|InputAxisGas
  (params (AxisValue :type Float%20%28single-precision%29))
  (Class|ChaosVehicleMovementComponent|SetThrottleInput (Variables|Default|GetVehicleMovementComponent) AxisValue))

(event Input|AxisEvents|InputAxisBremza
  (params (AxisValue :type Float%20%28single-precision%29))
  (Class|ChaosVehicleMovementComponent|SetBrakeInput (Variables|Default|GetVehicleMovementComponent) AxisValue))

(event Input|AxisEvents|InputAxisZavijanje
  (params (AxisValue :type Float%20%28single-precision%29))
  (Class|ChaosVehicleMovementComponent|SetSteeringInput (Variables|Default|GetVehicleMovementComponent) AxisValue))

(event Input|MouseEvents|MouseX
  (params (AxisValue :type Float%20%28single-precision%29))
  (Transformation|AddRelativeRotation (Variables|Default|GetSpringArm) (Math|Rotator|MakeRotator 0.0 0.0 AxisValue) false false))

(event Input|MouseEvents|MouseY
  (params (AxisValue :type Float%20%28single-precision%29))
  (Transformation|AddRelativeRotation (Variables|Default|GetSpringArm) (Math|Rotator|MakeRotator 0.0 AxisValue 0.0) false false))

(event Input|KeyboardEvents|M
  (params (Key :type Key%20Structure :default "None"))
  (:Pressed
    (bind _isa (Utilities|FlowControl|FlipFlop)
      (:A
        _)
      (:B
        _))
    (if _isa
      (Widget|SetVisibility (Variables|Default|GetMapcaUI) "Visible")
      (Audio|Components|Audio|Play (Variables|Default|GetmotorNoise) 0.0)
      (else
        (Widget|SetVisibility (Variables|Default|GetMapcaUI) "Collapsed")))))

(fn ConstructionScript)

(fn NovaMisija
  (params (TrenutnaMisija :type String))
  (Variables|Default|SetTrenutnaMisija TrenutnaMisija)
  (Rendering|Components|TextRender|SetText (Variables|/Game/dostave/DostaveTXTWidget.DostaveTXTWidget_C|GetTrenutnaDostava (Variables|Default|GetDostavaWidget)) (Utilities|Text|ToText(String) (Variables|Default|GetTrenutnaMisija))))

(fn Pretvori)

(fn DialogZac)